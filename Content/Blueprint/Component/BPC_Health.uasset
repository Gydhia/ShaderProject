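; BPC_Health is a health component that tracks an actor's HP and death state.
; HP starts at MaxHP on BeginPlay, and the ChangeHealth event adds a signed amount through SetLife, clamped between zero and MaxHP.
; After each change, CheckDeath sets IsDead when HP is zero and calls OnDeath.
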(event Custom|ChangeHealth
  (params (Damage%20Quantity :type Integer))
  (CallFunction|SetLife Damage%20Quantity))

(event EventBeginPlay
  (Variables|Default|SetHP (Variables|Default|GetMaxHP))
  (Development|PrintString "Start health"))

(event EventTick
  (params (DeltaSeconds :type Float%20%28single-precision%29)))

(fn SetLife
  (params (HPValue :type Integer))
  (Variables|Default|SetHP (Math|Integer|Clamp(Integer) (+ HPValue (Variables|Default|GetHP)) 0 (Variables|Default|GetMaxHP)))
  (CallFunction|CheckDeath)
  (return))

(fn CheckDeath
  (bind _output_get (Variables|Default|SetIsDead (== (Variables|Default|GetHP) 0)))
  (if _output_get
    (Default|CallOnDeath)))