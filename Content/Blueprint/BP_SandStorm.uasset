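; BP_SandStorm is a sandstorm effect actor that fades in on spawn and stays centered on the player.
; On BeginPlay, a timeline scaled by Seconds drives the mesh material's appear alpha.
; Each Tick moves the actor to the player and feeds materials the player position, plus a circle radius derived from the player's Sphere mesh bounds and size when that sphere is valid.
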(event EventBeginPlay
  (Components|Timeline|SetPlayRate (Variables|Default|GetTimeline) (/ 1.0 (Variables|Default|GetSeconds)))
  (bind _newtrack_0 (Timeline|Timeline PlayFromStart)
    (:Update
      (Rendering|Material|SetScalarParameterValueonMaterials (Variables|Debug|GetStaticMeshComponent) "_AppearAlpha" _newtrack_0))))

(event Collision|EventActorBeginOverlap
  (params (OtherActor :type Actor%20Object%20Reference)))

(event EventTick
  (params (DeltaSeconds :type Float%20%28single-precision%29))
  (bind _player (Variables|Default|GetPlayer))
  (bind _sphere (Variables|/Game/Blueprint/BP_MikeBis.BP_MikeBis_C|GetSphere _player))
  (bind _staticmeshcomponent (Variables|/Script/Engine.StaticMeshActor|GetStaticMeshComponent _sphere))
  (bind (_min _max) (Components|StaticMesh|GetLocalBounds _staticmeshcomponent))
  (Transformation|SetActorLocation (Transformation|GetActorLocation _player) false false)
  (Rendering|Material|SetVectorParameterValueonMaterials (Variables|Debug|GetStaticMeshComponent) "_PlayerPosition" (Transformation|GetActorLocation _player))
  (Utilities|IsValid _sphere
    (:Is%20Valid
      (Rendering|Material|SetScalarParameterValueonMaterials (Variables|Debug|GetStaticMeshComponent) "_CircleRadius" (/ (* (- (.x _max) (.x _min)) (Variables|/Game/Blueprint/BP_AirSphere.BP_AirSphere_C|GetSize _sphere)) 2.0)))))

(fn ConstructionScript)