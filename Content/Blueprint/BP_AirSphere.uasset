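; BP_AirSphere is a sphere actor that follows the referenced Player, repositioned every tick to a point slightly below the player's location.
; SetSize stores a new Size, scales the static mesh uniformly and writes the given alpha to the _AlphaAppear material parameter.
; BeginPlay calls SetSize with the current Size and zero alpha; nothing in this Blueprint assigns Player or changes the alpha afterward.
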(event EventBeginPlay
  (CallFunction|SetSize (Variables|Default|GetSize) 0.0))

(event Collision|EventActorBeginOverlap
  (params (OtherActor :type Actor%20Object%20Reference)))

(event EventTick
  (params (DeltaSeconds :type Float%20%28single-precision%29))
  (bind _player (Variables|Default|GetPlayer))
  (bind _returnvalue (Transformation|GetActorLocation _player))
  (Transformation|SetActorLocation (Math|Vector|MakeVector (.x _returnvalue) (.y _returnvalue) (- (.z _returnvalue) 1e+02)) false false))

(fn ConstructionScript)

(fn SetSize
  (params (newSize :type Float%20%28double-precision%29) (alpha :type Float%20%28double-precision%29))
  (Variables|Default|SetSize newSize)
  (Transformation|SetRelativeScale3D (Variables|Debug|GetStaticMeshComponent) (* (Class|KismetMathLibrary|VectorOne) (Variables|Default|GetSize)))
  (Rendering|Material|SetScalarParameterValueonMaterials (Variables|Debug|GetStaticMeshComponent) "_AlphaAppear" alpha))