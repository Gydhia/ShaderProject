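; BP_ZonePreview is an actor that shows a zone preview as a cylinder, in the casting preview folder.
; It has no active event logic and exposes functions to toggle, move and resize the Cylinder component.
; Visibility runs through the material's Fade scalar, where enabling sets zero and disabling sets one, or a caller supplies the value directly.
; SetHeight converts a height into Z scale against a fixed base and resets X and Y scale.
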(event EventBeginPlay)

(event Collision|EventActorBeginOverlap
  (params (OtherActor :type Actor%20Object%20Reference)))

(event EventTick
  (params (DeltaSeconds :type Float%20%28single-precision%29)))

(fn ConstructionScript)

(fn EnableZonePreview
  (params (Enable :type Boolean))
  (bind _cylinder (Variables|Default|GetCylinder))
  (if Enable
    (Rendering|Material|SetScalarParameterValueonMaterials _cylinder "Fade" 0.0)
    (else
      (Rendering|Material|SetScalarParameterValueonMaterials _cylinder "Fade" 1.0))))

(fn MovetoLocation
  (params (NewLocation :type Vector))
  (Transformation|SetWorldLocation (Variables|Default|GetCylinder) NewLocation false false))

(fn SetFadeValue
  (params (FadePercent :type Float%20%28double-precision%29))
  (Rendering|Material|SetScalarParameterValueonMaterials (Variables|Default|GetCylinder) "Fade" FadePercent))

(fn SetHeight
  (params (Height :type Float%20%28double-precision%29))
  (Transformation|SetWorldScale3D (Variables|Default|GetCylinder) (Math|Vector|MakeVector 1.0 1.0 (/ Height 8e+02))))